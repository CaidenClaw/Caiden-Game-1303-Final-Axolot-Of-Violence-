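; Game mode that runs a round-based enemy wave loop with upgrade intermissions.
; Each round spawns BP_EnemyAI at random BP_EnemySpawn points, in numbers that grow linearly with the round count.
; Tick polls for surviving enemies and, while none remain, calls the intermission every frame, attempting health and damage upgrade box spawns at their markers.
; After a fixed delay, it destroys both box types and starts the next round.
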(event Custom|StartIntermission
  (CallFunction|SpawnHealthUpgrade)
  (CallFunction|SpawnDamageUpgrade)
  (Utilities|FlowControl|Delay 1e+01)
  (CallFunction|EndIntermission))

(event Custom|End%20Intermission
  (CallFunction|DestroyUpgradeBox)
  (CallFunction|NextRound))

(event EventBeginPlay
  (CallFunction|NextRound))

(event EventTick
  (params (DeltaSeconds :type Float%20%28single-precision%29))
  (bind _outactors (Actor|GetAllActorsOfClass "/Game/FinalGame/Blueprints/Enemy/BP_EnemyAI.BP_EnemyAI_C"))
  (if (== (Utilities|Array|Length _outactors) 0)
    (CallFunction|StartIntermission)))

(fn ConstructionScript)

(fn NextRound
  (Variables|Default|SetCurrentRound (+ (Variables|Default|GetCurrentRound) 1))
  (Variables|Default|SetEnemySpawnAmount (+ (Variables|Default|GetBaseEnemySpawnAmount) (* (Variables|Default|GetCurrentRound) (Variables|Default|GetIncrement))))
  (for _index (range 0 (Variables|Default|GetEnemySpawnAmount))
    (bind _outactors (Actor|GetAllActorsOfClass "/Game/FinalGame/Blueprints/BP_EnemySpawn.BP_EnemySpawn_C"))
    (Game|SpawnActorfromClass "/Game/FinalGame/Blueprints/Enemy/BP_EnemyAI.BP_EnemyAI_C" (Transformation|GetActorTransform (.OutItem (Utilities|Array|Random _outactors))) "AdjustIfPossibleButAlwaysSpawn" "MultiplyWithRoot" 0 0)))

(fn SpawnHealthUpgrade
  (bind _returnvalue (Actor|GetActorOfClass "/Game/FinalGame/Blueprints/BP_HealthUpgradeSpawn.BP_HealthUpgradeSpawn_C"))
  (Game|SpawnActorfromClass "/Game/FinalGame/Blueprints/BP_UpgradeBox.BP_UpgradeBox_C" (Transformation|GetActorTransform _returnvalue) "DontSpawnIfColliding" "MultiplyWithRoot" 0 0))

(fn SpawnDamageUpgrade
  (bind _returnvalue (Actor|GetActorOfClass "/Game/FinalGame/Blueprints/BP_DamageUpgradeSpawn.BP_DamageUpgradeSpawn_C"))
  (Game|SpawnActorfromClass "/Game/FinalGame/Blueprints/BP_DamageUpgradeBox.BP_DamageUpgradeBox_C" (Transformation|GetActorTransform _returnvalue) "DontSpawnIfColliding" "MultiplyWithRoot" 0 0))

(fn DestroyUpgradeBox
  (Utilities|FlowControl|Sequence
    (:then_0
      (bind _outactors (Actor|GetAllActorsOfClass "/Game/FinalGame/Blueprints/BP_UpgradeBox.BP_UpgradeBox_C"))
      (Actor|DestroyActor _outactors))
    (:then_1
      (bind _outactors_2 (Actor|GetAllActorsOfClass "/Game/FinalGame/Blueprints/BP_DamageUpgradeBox.BP_DamageUpgradeBox_C"))
      (Actor|DestroyActor _outactors_2))))