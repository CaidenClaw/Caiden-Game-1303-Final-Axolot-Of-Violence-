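; Enemy AI pawn that chases the player, shoots on sight and awards points when killed.
; AI MoveTo targets the player character from BeginPlay and restarts only on success, while Tick refreshes the stored player position.
; PawnSensing spawns a projectile at ProjectileSpawn after a delay whenever it sees any pawn.
; Damage feeds BPHealth's DamageManager, whose true result adds points to BP_PlayerCharacter and destroys the enemy.
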(event OnSeePawn(PawnSensing)
  (params (Pawn :type Pawn%20Object%20Reference))
  (Utilities|FlowControl|Delay 1.5)
  (Game|SpawnActorfromClass "/Game/FinalGame/Blueprints/Enemy/BP_EnemyProjectile.BP_EnemyProjectile_C" (Transformation|GetWorldTransform (Variables|Default|GetProjectile%20Spawn)) "Undefined" "MultiplyWithRoot" 0 self)
  (Utilities|FlowControl|Delay 1.5)
  (Development|PrintString "I see you"))

(event Custom|MoveToPlayer
  (AI|AIMoveTo self (Variables|Default|GetPlayerPosition) (Game|GetPlayerCharacter 0) 5.0 false
    (:OnSuccess
      (CallFunction|MovetoPlayer))))

(event Custom|GetPlayerPosition
  (Variables|Default|SetPlayerPosition (Transformation|GetActorLocation (Game|GetPlayerCharacter 0))))

(event EventBeginPlay
  (CallFunction|MovetoPlayer))

(event Game|Damage|EventAnyDamage
  (params (Damage :type Float%20%28single-precision%29) (DamageType :type Damage%20Type%20Object%20Reference) (InstigatedBy :type Controller%20Object%20Reference) (DamageCauser :type Actor%20Object%20Reference))
  (bind _ishealthzero (Default|DamageManager (Variables|Default|GetBP_Health) Damage))
  (if _ishealthzero
    (bind _asbp_player_character (Utilities|Casting|CastToBP_PlayerCharacter (Game|GetPlayerCharacter 0)))
    (Default|AddPoints _asbp_player_character 5)
    (Actor|DestroyActor)))

(event EventTick
  (params (DeltaSeconds :type Float%20%28single-precision%29))
  (CallFunction|GetPlayerPosition))

(fn ConstructionScript)