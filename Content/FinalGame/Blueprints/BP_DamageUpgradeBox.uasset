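; BP_DamageUpgradeBox is a trigger-based shop pickup that sells the player a damage upgrade for points.
; On BeginPlay it caches the player 0 character as BP_PlayerCharacter.
; When that character overlaps CollisionTrigger with at least UpgradeCost points, it deducts the cost and calls UpgradeDamage on the character.
; Otherwise it prints a taunt, and the box stays in place for repeat purchases.
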(event OnComponentBeginOverlap(CollisionTrigger)
  (params (OverlappedComponent :type Primitive%20Component%20Object%20Reference) (OtherActor :type Actor%20Object%20Reference) (OtherComp :type Primitive%20Component%20Object%20Reference) (OtherBodyIndex :type Integer) (bFromSweep :type Boolean) (SweepResult :type Hit%20Result%20Structure%20%28by%20ref%29))
  (if (== OtherActor (Variables|Default|GetAs%20BP%20Player%20Character))
    (if (>= (Variables|/Game/FinalGame/Blueprints/Player/BP_PlayerCharacter.BP_PlayerCharacter_C|GetPoints (Variables|Default|GetAs%20BP%20Player%20Character)) (Variables|Default|GetUpgradeCost))
      (Default|RemovePoints (Variables|Default|GetAs%20BP%20Player%20Character) (Variables|Default|GetUpgradeCost))
      (Default|UpgradeDamage (Variables|Default|GetAs%20BP%20Player%20Character))
      (else
        (Development|PrintString "You're poor")))))

(event EventBeginPlay
  (bind _asbp_player_character (Utilities|Casting|CastToBP_PlayerCharacter (Game|GetPlayerCharacter 0)))
  (Variables|Default|SetAs%20BP%20Player%20Character _asbp_player_character))

(fn ConstructionScript)