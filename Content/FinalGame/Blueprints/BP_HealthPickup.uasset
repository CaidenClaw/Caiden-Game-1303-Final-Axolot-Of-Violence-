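; BP_HealthPickup is a pickup actor that restores a small fixed amount of the player's health.
; On BeginPlay it caches player 0's BP_PlayerCharacter, and only that actor overlapping PickupRadius can trigger it.
; If health is below maximum, it adds the amount clamped to max, refreshes the BPHealth component's health bar and destroys itself.
; Helper functions wrap access to BPHealth's current and maximum values.
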(event OnComponentBeginOverlap(PickupRadius)
  (params (OverlappedComponent :type Primitive%20Component%20Object%20Reference) (OtherActor :type Actor%20Object%20Reference) (OtherComp :type Primitive%20Component%20Object%20Reference) (OtherBodyIndex :type Integer) (bFromSweep :type Boolean) (SweepResult :type Hit%20Result%20Structure%20%28by%20ref%29))
  (if (== OtherActor (Variables|Default|GetAs%20BP%20Player%20Character))
    (if (< (Utilities|GetCurrentHealth) (Utilities|GetMaxHealth))
      (Utilities|SetCurrentHealth (Math|Float|Clamp(Float) (+ (Utilities|GetCurrentHealth) 1e+01) 0.0 (Utilities|GetMaxHealth)))
      (Default|UpdateHealthBar (Variables|/Game/FinalGame/Blueprints/Player/BP_PlayerCharacter.BP_PlayerCharacter_C|GetBP_Health (Variables|Default|GetAs%20BP%20Player%20Character)))
      (Actor|DestroyActor))))

(event EventBeginPlay
  (bind _asbp_player_character (Utilities|Casting|CastToBP_PlayerCharacter (Game|GetPlayerCharacter 0)))
  (Variables|Default|SetAs%20BP%20Player%20Character _asbp_player_character))

(fn ConstructionScript)